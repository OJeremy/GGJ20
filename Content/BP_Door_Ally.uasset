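; Door Blueprint that opens for allies, sliding vertically when an AllyCharacter enters its Box trigger.
; Overlap events track allies in PlayersDetected, using an exact class match on entry.
; The Opening_TL timeline lowers the Door's relative Z as it plays, and reverses to close once that list is empty.
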(event OnComponentBeginOverlap(Box)
  (params (OverlappedComponent :type Primitive%20Component%20Object%20Reference) (OtherActor :type Actor%20Object%20Reference) (OtherComp :type Primitive%20Component%20Object%20Reference) (OtherBodyIndex :type Integer) (bFromSweep :type Boolean) (SweepResult :type Hit%20Result%20Structure%20%28by%20ref%29))
  ;[1 1 1] Detect
  (if (== (Utilities|GetClass OtherActor) "/Game/ThirdPersonBase/ThirdPersonBP/AllyCharacter/AllyCharacter.AllyCharacter_C")
    (Utilities|Array|Add (Variables|Default|GetPlayersDetected) OtherActor)
    (Variables|Default|SetOpen? true)
    ;[1 1 1] OpeningSeq
    (bind _opening0_1 (Timeline|Opening_TL Play)
      (:Update
        (Transformation|SetRelativeLocation (Variables|Default|GetDoor) (Math|Vector|MakeVector 0.0 0.0 (Math|Float|MapRangeClamped _opening0_1 0.0 1.0 92.0 -126.0)) false false)))))

(event OnComponentEndOverlap(Box)
  (params (OverlappedComponent :type Primitive%20Component%20Object%20Reference) (OtherActor :type Actor%20Object%20Reference) (OtherComp :type Primitive%20Component%20Object%20Reference) (OtherBodyIndex :type Integer))
  ;[1 1 1] Detect
  (Utilities|Array|RemoveItem (Variables|Default|GetPlayersDetected) OtherActor)
  (if (== (Utilities|Array|Length (Variables|Default|GetPlayersDetected)) 0)
    (Variables|Default|SetOpen? false)
    ;[1 1 1] OpeningSeq
    (bind _opening0_1 (Timeline|Opening_TL Reverse)
      (:Update
        (Transformation|SetRelativeLocation (Variables|Default|GetDoor) (Math|Vector|MakeVector 0.0 0.0 (Math|Float|MapRangeClamped _opening0_1 0.0 1.0 92.0 -126.0)) false false)))))

(fn ConstructionScript
  (|CallParentFunction)
  (if (Variables|Default|GetOpen?)
    _))