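; BP_RepairPlayer is an interaction actor that lets one player revive the AllyCharacter it is parented to.
; On BeginPlay its sphere is set to ignore the parent actor when moving.
; Each activation adds a fixed revive amount to the parent, then copies the revive status to the instigating ally, flags it as reviving and updates that ally's QTE progress widget, showing it on screen if needed.
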(event EventBeginPlay
  (Collision|IgnoreActorwhenMoving (Variables|Default|GetSphere) (Actor|GetParentActor) true))

(event EventActivate
  (params (Instigator :type Pawn%20Object%20Reference))
  (bind _asally_character (Utilities|Casting|CastToAllyCharacter (Actor|GetParentActor)))
  (Default|Revive _asally_character 5 Instigator)
  (bind _asally_character_2 (Utilities|Casting|CastToAllyCharacter Instigator))
  (Variables|/Game/ThirdPersonBase/ThirdPersonBP/AllyCharacter/AllyCharacter.AllyCharacter_C|SetRevive_Progression _asally_character_2 (Variables|/Game/ThirdPersonBase/ThirdPersonBP/AllyCharacter/AllyCharacter.AllyCharacter_C|GetRevive_Status _asally_character))
  (Variables|/Game/ThirdPersonBase/ThirdPersonBP/AllyCharacter/AllyCharacter.AllyCharacter_C|SetIsReviving? _asally_character_2 true)
  (Default|UpdateProgress (Variables|/Game/ThirdPersonBase/ThirdPersonBP/AllyCharacter/AllyCharacter.AllyCharacter_C|GetQTEWidget _asally_character_2))
  (if (not (UserInterface|Viewport|IsinViewport (Variables|/Game/ThirdPersonBase/ThirdPersonBP/AllyCharacter/AllyCharacter.AllyCharacter_C|GetQTEWidget _asally_character_2)))
    (UserInterface|Viewport|AddtoPlayerScreen (Variables|/Game/ThirdPersonBase/ThirdPersonBP/AllyCharacter/AllyCharacter.AllyCharacter_C|GetQTEWidget _asally_character_2))))

(fn ConstructionScript
  (|CallParentFunction))