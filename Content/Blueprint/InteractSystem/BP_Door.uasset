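; Automatic two-panel door that opens when an enemy or ally character enters its trigger box.
; A timeline slides the panels apart vertically in opposite directions, with open and close sounds played in 2D.
; Detected characters are tracked in an array, and a DoOnce re-armed when the timeline finishes gates end-overlap handling.
; The timeline reverses to close the door once the array empties.
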(event OnComponentBeginOverlap(Box)
  (params (OverlappedComponent :type Primitive%20Component%20Object%20Reference) (OtherActor :type Actor%20Object%20Reference) (OtherComp :type Primitive%20Component%20Object%20Reference) (OtherBodyIndex :type Integer) (bFromSweep :type Boolean) (SweepResult :type Hit%20Result%20Structure%20%28by%20ref%29))
  (bind _returnvalue (Utilities|GetClass OtherActor))
  ;[1 1 1] Detect
  (if (or (== _returnvalue "/Game/ThirdPersonBase/ThirdPersonBP/EnemyCharacter/EnemyCharacter.EnemyCharacter_C") (== _returnvalue "/Game/ThirdPersonBase/ThirdPersonBP/AllyCharacter/AllyCharacter.AllyCharacter_C"))
    (Utilities|Array|Add (Variables|Default|GetPlayersDetected) OtherActor)
    (Variables|Default|SetOpen? true)
    ;[1 1 1] OpeningSeq
    (Audio|PlaySound2D "/Game/Son/SD_OPENDOOR_Cue.SD_OPENDOOR_Cue" 1.0 1.0 0.0 0 0)
    (bind _opening0_1 (Timeline|Opening_TL Play)
      (:Update
        (Utilities|FlowControl|Sequence
          (:then_0
            (Transformation|SetRelativeLocation (Variables|Default|Getporte_porte1) (Math|Vector|MakeVector 0.0 0.0 (Math|Float|MapRangeClamped _opening0_1 0.0 1.0 0.0 1.8e+02)) false false))
          (:then_1
            (Transformation|SetRelativeLocation (Variables|Default|Getporte_porte) (Math|Vector|MakeVector 0.0 0.0 (Math|Float|MapRangeClamped _opening0_1 0.0 1.0 0.0 -1.8e+02)) false false))))
      (:Finished
        (Utilities|FlowControl|DoOnce false) ; enters at Reset
      ))))

(event OnComponentEndOverlap(Box)
  (params (OverlappedComponent :type Primitive%20Component%20Object%20Reference) (OtherActor :type Actor%20Object%20Reference) (OtherComp :type Primitive%20Component%20Object%20Reference) (OtherBodyIndex :type Integer))
  ;[1 1 1] Detect
  (Utilities|FlowControl|DoOnce false :!label _label
    (:Completed
      (Utilities|Array|RemoveItem (Variables|Default|GetPlayersDetected) OtherActor)
      (if (== (Utilities|Array|Length (Variables|Default|GetPlayersDetected)) 0)
        (Variables|Default|SetOpen? false)
        ;[1 1 1] OpeningSeq
        (Audio|PlaySound2D "/Game/Son/SD_CLOSEDOOR_Cue.SD_CLOSEDOOR_Cue" 1.0 1.0 0.0 0 0)
        (bind _opening0_1 (Timeline|Opening_TL Reverse)
          (:Update
            (Utilities|FlowControl|Sequence
              (:then_0
                (Transformation|SetRelativeLocation (Variables|Default|Getporte_porte1) (Math|Vector|MakeVector 0.0 0.0 (Math|Float|MapRangeClamped _opening0_1 0.0 1.0 0.0 1.8e+02)) false false))
              (:then_1
                (Transformation|SetRelativeLocation (Variables|Default|Getporte_porte) (Math|Vector|MakeVector 0.0 0.0 (Math|Float|MapRangeClamped _opening0_1 0.0 1.0 0.0 -1.8e+02)) false false))))
          (:Finished
            (goto _label Reset)))
        (else
          (goto _label Reset))))))

(fn ConstructionScript
  (|CallParentFunction)
  (if (Variables|Default|GetOpen?)
    _))