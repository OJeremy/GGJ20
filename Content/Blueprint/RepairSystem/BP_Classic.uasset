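; BP_Classic is a repairable object in the repair system that swaps its static mesh based on health.
; Activate adds the repair value to HP0 if health is non-negative and below maximum, clamping to a fixed 100 rather than MaxHP0.
; It prints the result, then a truncated range map selects MeshHP100 below half of MaxHP0, otherwise MeshHP50.
; The construction script calls its parent and starts with MeshHP100.
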(event EventActivate
  (params (RepearValue :type Integer))
  (if (and (< (Variables|Default|GetHP_0) (Variables|Default|GetMaxHP_0)) (>= (Variables|Default|GetHP_0) 0))
    (bind _output_get (Variables|Default|SetHP_0 (Math|Integer|Clamp(Integer) (+ (Variables|Default|GetHP_0) RepearValue) 0 100)))
    (Development|PrintString (Utilities|String|ToString(Integer) _output_get))
    (Components|StaticMesh|SetStaticMesh (Variables|Default|GetMesh) (Utilities|Select :Index (Math|Float|Truncate (Math|Float|MapRangeClamped (Math|Conversions|ToFloat(Integer) (Variables|Default|GetHP_0)) 0.0 (Math|Conversions|ToFloat(Integer) (/ (Variables|Default|GetMaxHP_0) 2)) 0.0 1.0)) :Option%200 (Variables|Default|GetMesh_HP100) :Option%201 (Variables|Default|GetMesh_HP50)))))

(fn ConstructionScript
  (|CallParentFunction)
  (Components|StaticMesh|SetStaticMesh (Variables|Default|GetMesh) (Variables|Default|GetMesh_HP100)))