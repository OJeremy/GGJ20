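; BP_Destructible is a repair-system piece whose HP can be damaged or repaired, with a valid state and mesh to match.
; Activate adds a signed value to clamped HP, sounds an alarm and disables the piece when damaged at zero HP, and ignores further damage until repaired.
; HP thresholds swap damaged and intact meshes, with a DoOnce limiting the repaired sound to once per repair.
; BrokeDevice breaks it instantly, and construction derives validity from HP.
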(event Custom|BrokeDevice
  (Variables|Default|SetHP 0)
  (Components|StaticMesh|SetStaticMesh (Variables|Default|GetMesh) (Variables|Default|GetMesh_HP50))
  (Variables|Default|SetValidPiece false))

(event EventActivate
  (params (RepearValue :type Integer))
  (bind _mesh (Variables|Default|GetMesh))
  (if (and (<= (Variables|Default|GetHP) (Variables|Default|GetMaxHP)) (>= (Variables|Default|GetHP) 0))
    (if (< RepearValue 0)
      (if (not (Variables|Default|GetDisabled))
        (if (== 0 (Variables|Default|GetHP))
          (Audio|PlaySound2D "/Game/Son/Already_Add/SFX_LayerAlarm_Cue.SFX_LayerAlarm_Cue" 1.0 1.0 0.0 0 0)
          (Variables|Default|SetDisabled true)
          (else
            (Utilities|FlowControl|Sequence :!label _label
              (:then_0
                (Variables|Default|SetDisabled false)))))
        (bind _output_get (Variables|Default|SetHP (Math|Integer|Clamp(Integer) (+ (Variables|Default|GetHP) RepearValue) 0 100)))
        (if (< _output_get 99)
          (Variables|Default|SetValidPiece false)
          (Components|StaticMesh|SetStaticMesh _mesh (Variables|Default|GetMesh_HP50))
          (goto _label_2 Reset)
          (else
            (Variables|Default|SetValidPiece true)
            (Components|StaticMesh|SetStaticMesh _mesh (Variables|Default|GetMesh_HP100))
            (Utilities|FlowControl|DoOnce false :!label _label_2
              (:Completed
                (Audio|PlaySound2D "/Game/Son/Already_Add/SFX_Blue_Repaired_Cue.SFX_Blue_Repaired_Cue" 1.0 1.0 0.0 0 0))))))
      (else
        (goto _label)))))

(fn ConstructionScript
  (|CallParentFunction)
  (if (< (Variables|Default|GetHP) 100)
    (Variables|Default|SetValidPiece false)
    (else
      (Variables|Default|SetValidPiece true))))