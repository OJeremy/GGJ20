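; BP_RepairMaster is a repairable-object Blueprint, apparently meant as a base for the repair system.
; Its Sphere component adds the actor to an overlapping AllyCharacter's or EnemyCharacter's ReparableInRange list and removes it when the overlap ends.
; The Activate event takes a repair value but has no logic here.
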(event OnComponentBeginOverlap(Sphere)
  (params (OverlappedComponent :type Primitive%20Component%20Object%20Reference) (OtherActor :type Actor%20Object%20Reference) (OtherComp :type Primitive%20Component%20Object%20Reference) (OtherBodyIndex :type Integer) (bFromSweep :type Boolean) (SweepResult :type Hit%20Result%20Structure%20%28by%20ref%29))
  (bind _asally_character (Utilities|Casting|CastToAllyCharacter OtherActor)
    (:then
      (Utilities|Array|Add (Variables|/Game/ThirdPersonBase/ThirdPersonBP/AllyCharacter/AllyCharacter.AllyCharacter_C|GetReparableInRange _asally_character) self))
    (:CastFailed
      (bind _asenemy_character (Utilities|Casting|CastToEnemyCharacter OtherActor))
      (Utilities|Array|Add (Variables|/Game/ThirdPersonBase/ThirdPersonBP/EnemyCharacter/EnemyCharacter.EnemyCharacter_C|GetReparableInRange _asenemy_character) self))))

(event OnComponentEndOverlap(Sphere)
  (params (OverlappedComponent :type Primitive%20Component%20Object%20Reference) (OtherActor :type Actor%20Object%20Reference) (OtherComp :type Primitive%20Component%20Object%20Reference) (OtherBodyIndex :type Integer))
  (bind _asally_character (Utilities|Casting|CastToAllyCharacter OtherActor)
    (:then
      (Utilities|Array|RemoveItem (Variables|/Game/ThirdPersonBase/ThirdPersonBP/AllyCharacter/AllyCharacter.AllyCharacter_C|GetReparableInRange _asally_character) self))
    (:CastFailed
      (bind _asenemy_character (Utilities|Casting|CastToEnemyCharacter OtherActor))
      (Utilities|Array|RemoveItem (Variables|/Game/ThirdPersonBase/ThirdPersonBP/EnemyCharacter/EnemyCharacter.EnemyCharacter_C|GetReparableInRange _asenemy_character) self))))

(event Custom|Activate
  (params (RepearValue :type Integer)))

(fn ConstructionScript)