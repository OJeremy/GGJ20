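; BP_SpawnPoint is a spawn point actor for players that exposes where to spawn and whether spawning there is currently allowed.
; The construction script stores the world transform of its arrow component as SpawnCoords.
; The PlayerIsSpawning event clears CanSpawn, then restores it after a short delay, giving the point a cooldown between spawns.
; A debug print naming the point is present but unconnected.
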(event Custom|PlayerIsSpawning
  (Variables|Default|SetCanSpawn? false)
  (Utilities|FlowControl|Delay 2.0)
  (Variables|Default|SetCanSpawn? true))

(event EventBeginPlay)

(fn ConstructionScript
  (Variables|Default|SetSpawnCoords (Transformation|GetWorldTransform (Variables|Default|GetArrow_spawnPoint))))