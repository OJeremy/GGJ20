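; BP_GameLoop sets up both teams at BeginPlay, spawning and possessing local player characters at BP_SpawnPoint actors.
; For each character it claims the first available point matching the team.
; Player 0 gets an EnemyCharacter; after a short delay, a NumPlayers loop creates additional local players with AllyCharacters on the other team, varying mesh materials by index.
; The AllyTeamSpawn and EnemyTeamSpawn labels run opposite to those class names.
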(event EventBeginPlay
  (bind _outactors (Actor|GetAllActorsOfClass "/Game/Blueprint/GameCore/BP_SpawnPoint.BP_SpawnPoint_C"))
  (bind _output_get (Variables|Default|SetSpawnPoints _outactors))
  (if (> (Utilities|Array|Length _output_get) 0)
    (Utilities|FlowControl|Sequence
      (:then_0
        ;[1 1 1] AllyTeamSpawn
        (bind _array_element (Utilities|Array|ForEachLoopwithBreak (Variables|Default|GetSpawnPoints) :!label _label)
          (:LoopBody
            (if (and (Variables|/Game/Blueprint/GameCore/BP_SpawnPoint.BP_SpawnPoint_C|GetCanSpawn? _array_element) (Utilities|Enum|Equal(Enum) (Variables|/Game/Blueprint/GameCore/BP_SpawnPoint.BP_SpawnPoint_C|GetTeam _array_element) "NewEnumerator1"))
              (Default|PlayerIsSpawning _array_element)
              (goto _label Break)))
          (:Completed
            (bind _returnvalue (Game|SpawnActorfromClass "/Game/ThirdPersonBase/ThirdPersonBP/EnemyCharacter/EnemyCharacter.EnemyCharacter_C" (Variables|/Game/Blueprint/GameCore/BP_SpawnPoint.BP_SpawnPoint_C|GetSpawnCoords _array_element) "AlwaysSpawn" 0 1e+02 -5 0))
            (Default|SetTeam _returnvalue "NewEnumerator1")
            (Utilities|IsValid _returnvalue
              (:Is%20Valid
                (Pawn|Possess (Game|GetPlayerController 0) _returnvalue))))))
      (:then_1
        ;[1 1 1] EnemyTeamSpawn
        (Utilities|FlowControl|Delay 0.1)
        (for _index (range 0 (- (Variables|Default|GetNumPlayers) 1))
          (bind _returnvalue_2 (Class|GameplayStatics|CreatePlayer -1))
          (bind _array_element_2 (Utilities|Array|ForEachLoopwithBreak (Variables|Default|GetSpawnPoints) :!label _label_2)
            (:LoopBody
              (if (and (Variables|/Game/Blueprint/GameCore/BP_SpawnPoint.BP_SpawnPoint_C|GetCanSpawn? _array_element_2) (Utilities|Enum|Equal(Enum) (Variables|/Game/Blueprint/GameCore/BP_SpawnPoint.BP_SpawnPoint_C|GetTeam _array_element_2) "NewEnumerator0"))
                (Default|PlayerIsSpawning _array_element_2)
                (goto _label_2 Break)))
            (:Completed
              (bind _returnvalue_3 (Game|SpawnActorfromClass "/Game/ThirdPersonBase/ThirdPersonBP/AllyCharacter/AllyCharacter.AllyCharacter_C" (Variables|/Game/Blueprint/GameCore/BP_SpawnPoint.BP_SpawnPoint_C|GetSpawnCoords _array_element_2) "AlwaysSpawn" 0 0))
              (Default|SetTeam _returnvalue_3 "NewEnumerator0")
              (Rendering|Material|SetMaterial (Variables|/Script/Engine.Character|GetMesh _returnvalue_3) 0 (Utilities|Select :Index _index :Option%200 0 :Option%201 0 :Option%202 0))
              (Rendering|Material|SetMaterial (Variables|/Script/Engine.Character|GetMesh _returnvalue_3) 1 (Utilities|Select :Index _index :Option%200 0 :Option%201 0 :Option%202 0))
              (Pawn|Possess _returnvalue_2 _returnvalue_3))))))))

(fn ConstructionScript)